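; BP_Weight is a weight-sensitive object that fades out and destroys itself once it has registered at least three distinct pawns.
; A Character_Base overlap triggers, after a short delay, an upward box trace sized by actor scale, adding hit actors to a never-cleared unique list.
; At the threshold, a timeline drives Transparency on a dynamic galaxy material, then records its location in BP_WeightArea's WeightLocationRemoved before destruction.
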(event `self.Box.OnComponentBeginOverlap`
  (params (OverlappedComponent :type "PrimitiveComponent Object Reference") (OtherActor :type "Actor Object Reference") (OtherComp :type "PrimitiveComponent Object Reference") (OtherBodyIndex :type Integer) (bFromSweep :type Boolean) (SweepResult :type "HitResult Structure (by ref)"))
  (bind _returnvalue (`self.K2_GetActorLocation`))
  (bind (_returnvalue_location _returnvalue_rotation _returnvalue_scale) (`KismetMathLibrary.BreakTransform` (`self.GetTransform`)))
  (cast `/Game/Character/Character_Base` OtherActor)
  (`KismetSystemLibrary.Delay` 0.5)
  (bind _outhits (`KismetSystemLibrary.BoxTraceMultiForObjects` _returnvalue (+ _returnvalue (* (`self.GetActorUpVector`) 100.0)) (* _returnvalue_scale 50.0) (struct) (`|MakeArray` "ObjectTypeQuery3" :!type "EObjectTypeQuery Enum")))
  (for _array_element _outhits
    (`KismetArrayLibrary.Array_AddUnique` (`self.Hit Actor`) (`.HitActor` (`GameplayStatics.BreakHitResult` _array_element))))
  (if (>= (`KismetArrayLibrary.Array_Length` (`self.Hit Actor`)) 3)
    (bind (_direction `_新建轨道_0`) (`Timeline|时间轴` :!via `PlayFromStart`)
      (:`Update`
        (`MaterialInstanceDynamic.SetScalarParameterValue` (`self.Dynamic Material`) "Transparency" `_新建轨道_0`))
      (:`Finished`
        (bind _returnvalue_2 (`GameplayStatics.GetActorOfClass` "/Game/Character/Player2/BP_WeightArea.BP_WeightArea_C"))
        (`KismetArrayLibrary.Array_AddUnique` (`/Game/Character/Player2/BP_WeightArea.WeightLocation_Removed` _returnvalue_2) (`self.K2_GetActorLocation`))
        (`self.K2_DestroyActor`)))))

(fn `UserConstructionScript`
  (bind _returnvalue (`PrimitiveComponent.CreateDynamicMaterialInstance` (`self.StaticMesh`) 0 "/Game/Character/Player2/GalaxyMaterials/Resources/MaterialInstances/ForMeshes/MI_GalaxyMaterial_01.MI_GalaxyMaterial_01" "None"))
  (set `self.Dynamic Material` _returnvalue))