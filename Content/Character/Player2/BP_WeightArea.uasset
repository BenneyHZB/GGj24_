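; BP_WeightArea is an area actor that respawns BP_Weight actors at locations stored in WeightLocationRemoved.
; A Character_Base overlapping its Box sets PlyerEnter, which this graph never clears.
; A looping timer checks that flag and the list, then after a delay box-traces each location for Pawns.
; Unblocked locations get a new weight and are removed from the array during the loop over it.
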(event `self.ReceiveBeginPlay`
  (`KismetSystemLibrary.K2_SetTimerDelegate` (delegate `自定义事件`) 5.0 true))

(event `自定义事件`
  (if (and (`self.PlyerEnter?`) (`KismetArrayLibrary.Array_IsNotEmpty` (`self.WeightLocation_Removed`)))
    (`KismetSystemLibrary.Delay` 5.0)
    (for _array_element (`self.WeightLocation_Removed`)
      (bind (_outhit _returnvalue) (`KismetSystemLibrary.BoxTraceSingleForObjects` _array_element (+ _array_element (* (`self.GetActorUpVector`) 100.0)) (* (1.0 3.25 1.0) 50.0) (struct) (`|MakeArray` "ObjectTypeQuery3" :!type "EObjectTypeQuery Enum")))
      (if (not _returnvalue)
        (`|SpawnActorFromClass` "/Game/Character/Player2/BP_Weight.BP_Weight_C" (`KismetMathLibrary.MakeTransform` _array_element (struct) (1.0 3.25 1.0)) "Undefined" "MultiplyWithRoot" null null)
        (`KismetArrayLibrary.Array_RemoveItem` (`self.WeightLocation_Removed`) _array_element)))))

(event `self.Box.OnComponentBeginOverlap`
  (params (OverlappedComponent :type "PrimitiveComponent Object Reference") (OtherActor :type "Actor Object Reference") (OtherComp :type "PrimitiveComponent Object Reference") (OtherBodyIndex :type Integer) (bFromSweep :type Boolean) (SweepResult :type "HitResult Structure (by ref)"))
  (cast `/Game/Character/Character_Base` OtherActor)
  (set `self.PlyerEnter?` true))

(fn `UserConstructionScript`)