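; BP_TouchDead_Move is a moving touch hazard that kills characters entering its Box collision.
; Tick accumulates elapsed time in YMove and adds a local Y offset of its sine times Distance each frame, so the back-and-forth travel depends on frame rate.
; A Box overlap with a Character_Base destroys that character after a short delay.
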(event `self.ReceiveTick`
  (params (DeltaSeconds :type "Float (single-precision)"))
  (bind _output_get (set `self.Y Move` (+ DeltaSeconds (`self.Y Move`))))
  (`self.K2_AddActorLocalOffset` (`KismetMathLibrary.MakeVector` 0.0 (* (`KismetMathLibrary.Sin` _output_get) (`self.Distance`)))))

(event `self.Box.OnComponentBeginOverlap`
  (params (OverlappedComponent :type "PrimitiveComponent Object Reference") (OtherActor :type "Actor Object Reference") (OtherComp :type "PrimitiveComponent Object Reference") (OtherBodyIndex :type Integer) (bFromSweep :type Boolean) (SweepResult :type "HitResult Structure (by ref)"))
  (bind _ascharacter_base (cast `/Game/Character/Character_Base` OtherActor))
  (`KismetSystemLibrary.Delay` 0.3)
  (`self.K2_DestroyActor` _ascharacter_base))

(fn `UserConstructionScript`)